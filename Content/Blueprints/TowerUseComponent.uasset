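; Use component for a tower that lets a player build it or repair it through its HealComponent.
; On use, a working tower starts a fast looping timer, while an unbuilt one checks and deducts Diament, Brick and Wood once, then starts a slower one.
; Each build step heals a multiple of the repair value, notifying the tower at full HP.
; Stopping use clears the timer, and paid construction resumes without another charge.
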(event Custom|FixTower
  (Default|GetHeal (Variables|Default|GetHealComponentRef) (Variables|Default|GetReperValue)))

(event Custom|InitComponent
  (params (HealComponentRef :type Health%20Component%20Object%20Reference) (RefToTower :type Tower%20Object%20Reference))
  (Utilities|FlowControl|Sequence
    (:then_0
      (Variables|Default|SetHealComponentRef HealComponentRef))
    (:then_1
      (Variables|Default|SetRefToTower RefToTower))
    (:then_2
      (Variables|Default|SetBuildingValue (* (Variables|Default|GetReperValue) 4e+01)))))

(event Custom|BuildTower
  (bind _healcomponentref (Variables|Default|GetHealComponentRef))
  (Default|GetHeal (Variables|Default|GetHealComponentRef) (Variables|Default|GetBuildingValue))
  (Audio|PlaySound2D "/Game/Sound/mot.mot" 1.0 1.0 0.0 0 0)
  (if (>= (Variables|/Game/Blueprints/HealthComponent.HealthComponent_C|GetCurrenHP _healcomponentref) (Variables|/Game/Blueprints/HealthComponent.HealthComponent_C|GetMaxHP _healcomponentref))
    (Default|TowerHasBeenBuild (Variables|Default|GetRefToTower))
    (CallFunction|FStopUse)))

(fn FUsed
  (params (PlayerRef :type Third%20Person%20Character%20Object%20Reference))
  (bind _equipmentcomponent (Variables|/Game/Blueprints/Core/ThirdPersonCharacter.ThirdPersonCharacter_C|GetEquipmentComponent PlayerRef))
  (bind _reftotower (Variables|Default|GetRefToTower))
  (|CallParentFunction 0)
  (if (Variables|/Game/Blueprints/Tower.Tower_C|GetIsWorking (Variables|Default|GetRefToTower))
    (bind _returnvalue (Utilities|Time|SetTimerbyEvent (EventDispatchers|CreateEvent :!event Custom|FixTower) 0.1 true))
    (Variables|Default|SetUsingTimer _returnvalue)
    (elif (Variables|Default|GetHasBeenBuild)
      (CallFunction|BuildTower :!label _label)
      (bind _returnvalue_2 (Utilities|Time|SetTimerbyEvent (EventDispatchers|CreateEvent :!event Custom|BuildTower) 1.2 true))
      (Variables|Default|SetUsingTimer _returnvalue_2)
      (else
        (bind (_succes _deletthisitems) (CallFunction|CheakBuildRequest (Variables|/Game/Blueprints/EquipmentComponent.EquipmentComponent_C|GetBuildingItems _equipmentcomponent)))
        (if _succes
          (Default|DeletBuildingItems _equipmentcomponent _deletthisitems)
          (Rendering|SetVisibility (Variables|/Game/Blueprints/Tower.Tower_C|GetHealBar _reftotower) true false)
          (Variables|Default|SetHasBeenBuild true)
          (Rendering|SetVisibility (Variables|/Game/Blueprints/Tower.Tower_C|GetBuildRequest _reftotower) false false)
          (goto _label)
          (else
            (Development|PrintString "Not Enought Minnerals!!")))))))

(fn FStopUse
  (|CallParentFunction)
  (Utilities|Time|ClearandInvalidateTimerbyHandle (Variables|Default|GetUsingTimer)))

(fn CheakBuildRequest
  (params (Request :type Build%20Request%20Struct%20Structure))
  (bind _buildrequest (Variables|Default|GetBuildRequest))
  (return (Math|Boolean|ANDBoolean (>= (.diament Request) (.diament _buildrequest)) (>= (.brick Request) (.brick _buildrequest)) (>= (.wood Request) (.wood _buildrequest))) (Variables|Default|GetBuildRequest)))