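; Health component that tracks an owning actor's current and max HP, handling damage, healing and death.
; InitComponent starts from a custom HP value or fills to max, and each change updates WidgetHP and broadcasts the current HP.
; TakeDamage respects Immortal and IsLive, signaling death and returning true at zero.
; GetHeal adds HP without clamping to max and fires the max-HP event on every heal.
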(event Custom|InitComponent
  (params (SetUpCustomCurrentHP :type Boolean) (CustomHP :type Float%20%28single-precision%29))
  (if SetUpCustomCurrentHP
    (bind _output_get (Variables|Default|SetCurrenHP CustomHP))
    (Variables|/Game/Widgets/HealthBar.HealthBar_C|SetWidgetMax_HP (Variables|Default|GetWidgetHP) (Variables|Default|GetMaxHP))
    (Variables|/Game/Widgets/HealthBar.HealthBar_C|SetWidget_HP (Variables|Default|GetWidgetHP) _output_get)
    (Default|CallYourCurrentHP _output_get)
    (else
      (CallFunction|SetMaxHP))))

(fn TakeDamage
  (params (Damage :type Float%20%28single-precision%29))
  (if (and (Variables|Default|GetIsLive) (not (Variables|Default|GetImmortal)))
    (bind _output_get (Variables|Default|SetCurrenHP (- (Variables|Default|GetCurrenHP) Damage)))
    (bind _output_get_2 (Variables|/Game/Widgets/HealthBar.HealthBar_C|SetWidget_HP (Variables|Default|GetWidgetHP) _output_get))
    (Default|CallYourCurrentHP _output_get_2)
    (if (<= _output_get 0.0)
      (Variables|Default|SetIsLive false)
      (Variables|Default|SetCurrenHP 0.0)
      (Default|CallYouAreDead)
      (return true)
      (else
        (return false)))))

(fn SetMaxHP
  (Variables|Default|SetIsLive true)
  (bind _output_get (Variables|Default|SetCurrenHP (Variables|Default|GetMaxHP)))
  (Variables|/Game/Widgets/HealthBar.HealthBar_C|SetWidgetMax_HP (Variables|Default|GetWidgetHP) (Variables|Default|GetMaxHP))
  (bind _output_get_2 (Variables|/Game/Widgets/HealthBar.HealthBar_C|SetWidget_HP (Variables|Default|GetWidgetHP) _output_get))
  (Default|CallYourCurrentHP _output_get_2))

(fn GetHeal
  (params (Heal :type Float%20%28single-precision%29))
  (if (< (Variables|Default|GetCurrenHP) (Variables|Default|GetMaxHP))
    (bind _output_get (Variables|Default|SetCurrenHP (+ (Variables|Default|GetCurrenHP) Heal)))
    (bind _output_get_2 (Variables|/Game/Widgets/HealthBar.HealthBar_C|SetWidget_HP (Variables|Default|GetWidgetHP) _output_get))
    (Default|CallYourCurrentHP _output_get_2)
    (Default|CallYouHasMaxHP)
    (Development|PrintString (Utilities|String|Append (Utilities|GetObjectName (Components|GetOwner)) " has been heal to : " (Utilities|String|ToString(Float) (Variables|Default|GetCurrenHP))))))