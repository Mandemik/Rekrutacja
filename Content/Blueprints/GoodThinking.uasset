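; GoodThinking is a collectible memory that a ThirdPersonCharacter carries one at a time and later deploys.
; Box overlap triggers PickUp, which flags the carrier, plays a sound, calls Picked, hides the actor and binds to the player's death and DeployMemory dispatchers.
; Reset restores the pickup, while AddThisMemory passes the sphere mesh to DeployEnergy, adds image and text to the HUD book, then destroys the actor.
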(event OnComponentBeginOverlap(Box)
  (params (OverlappedComponent :type Primitive%20Component%20Object%20Reference) (OtherActor :type Actor%20Object%20Reference) (OtherComp :type Primitive%20Component%20Object%20Reference) (OtherBodyIndex :type Integer) (bFromSweep :type Boolean) (SweepResult :type Hit%20Result%20Structure%20%28by%20ref%29))
  (bind _asthird_person_character (Utilities|Casting|CastToThirdPersonCharacter OtherActor))
  (if (and (not (Variables|Default|GetHasBeenPick)) (not (Variables|/Game/Blueprints/Core/ThirdPersonCharacter.ThirdPersonCharacter_C|GetCarringMemory _asthird_person_character)))
    (CallFunction|PickUp _asthird_person_character)))

(fn ConstructionScript
  (|CallParentFunction))

(fn PickUp
  (params (PlayerRef :type Third%20Person%20Character%20Object%20Reference))
  (Variables|/Game/Blueprints/Core/ThirdPersonCharacter.ThirdPersonCharacter_C|SetCarringMemory PlayerRef true)
  (Variables|Default|SetHasBeenPick true)
  (Variables|Default|SetPlayerRef PlayerRef)
  (Audio|PlaySound2D "/Game/Sound/podnoszenie.podnoszenie" 1.0 1.0 0.0 0 0)
  (Default|CallPicked)
  (Rendering|SetActorHiddenInGame true)
  (EventDispatchers|BindEventtoYouAreDead (Variables|/Game/Blueprints/Core/ThirdPersonCharacter.ThirdPersonCharacter_C|GetHealthComponent PlayerRef) (EventDispatchers|CreateEvent :!event Reset))
  (EventDispatchers|BindEventtoDeployMemory PlayerRef (EventDispatchers|CreateEvent :!event AddThisMemory)))

(fn Reset
  (Variables|/Game/Blueprints/Core/ThirdPersonCharacter.ThirdPersonCharacter_C|SetCarringMemory (Variables|Default|GetPlayerRef) false)
  (Variables|Default|SetHasBeenPick false)
  (Rendering|SetActorHiddenInGame false))

(fn AddThisMemory
  (bind _playerref (Variables|Default|GetPlayerRef))
  (Variables|/Game/Blueprints/Core/ThirdPersonCharacter.ThirdPersonCharacter_C|SetCarringMemory _playerref false)
  (Default|DeployEnergy _playerref (Variables|/Script/Engine.StaticMeshComponent|GetStaticMesh (Variables|Default|GetSphere)))
  (Default|AddNewItem (Variables|/Game/Widgets/PlayerHud.PlayerHud_C|GetBookWIdget (Variables|/Game/Blueprints/Core/ThirdPersonCharacter.ThirdPersonCharacter_C|GetPlayerHUD _playerref)) (Variables|Default|GetTexture) (Variables|Default|GetText))
  (Actor|DestroyActor))