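; Player controller that turns player input into ThirdPersonCharacter actions and manages focus between gameplay and HUD widgets.
; It caches the pawn on BeginPlay, forwarding dash, use press/release and yaw-only, control-relative movement to it.
; Note and menu actions toggle HUD widgets, whose returned state drives SwitchControlToWidget to set cursor and input mode.
; Separate functions, not called here, hand focus fully to the main menu or back to gameplay.
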(event EventBeginPlay
  ;[0 0 0] Init
  (bind _asthird_person_character (Utilities|Casting|CastToThirdPersonCharacter (Pawn|GetControlledPawn)))
  (Variables|Default|SetPlayerRef _asthird_person_character))

(event Input|ActionEvents|InputActionDash
  (params (Key :type Key%20Structure :default "None"))
  (:Pressed
    (Default|Dash (Variables|Default|GetPlayerRef))))

(event Input|ActionEvents|InputActionOpenNote
  (params (Key :type Key%20Structure :default "None"))
  (bind _playerref (Variables|Default|GetPlayerRef))
  (bind _playerhud (Variables|/Game/Blueprints/Core/ThirdPersonCharacter.ThirdPersonCharacter_C|GetPlayerHUD _playerref))
  (:Pressed
    (bind _widgetactive_ (Default|SwitchWidget _playerhud))
    (CallFunction|SwitchControltoWidget _widgetactive_ (Variables|/Game/Widgets/PlayerHud.PlayerHud_C|GetBookWIdget _playerhud))))

(event Input|ActionEvents|InputActionUse
  (params (Key :type Key%20Structure :default "None"))
  (:Pressed
    (Default|UseComponent (Variables|Default|GetPlayerRef) true))
  (:Released
    (Default|UseComponent (Variables|Default|GetPlayerRef) false)))

(event Input|ActionEvents|InputActionOpen/CloseMenu
  (params (Key :type Key%20Structure :default "None"))
  (bind _playerref (Variables|Default|GetPlayerRef))
  (bind _playerhud (Variables|/Game/Blueprints/Core/ThirdPersonCharacter.ThirdPersonCharacter_C|GetPlayerHUD _playerref))
  (:Pressed
    (bind _menuopen_ (Default|OpenMainMenu _playerhud))
    (CallFunction|SwitchControltoWidget _menuopen_ _playerhud)))

(event Input|AxisEvents|InputAxisMoveForward
  (params (AxisValue :type Float%20%28single-precision%29))
  ;[0 0 0] Movement
  (Pawn|Input|AddMovementInput (Variables|Default|GetPlayerRef) (Math|Vector|GetForwardVector (Math|Rotator|MakeRotator 0.0 0.0 (.Yaw (Math|Rotator|BreakRotator (Pawn|GetControlRotation (Variables|Default|GetPlayerRef) :!class /Script/Engine.Pawn))))) AxisValue false))

(event Input|AxisEvents|InputAxisMoveRight
  (params (AxisValue :type Float%20%28single-precision%29))
  ;[0 0 0] Movement
  (Pawn|Input|AddMovementInput (Variables|Default|GetPlayerRef) (Math|Vector|GetRightVector (Math|Rotator|MakeRotator 0.0 0.0 (.Yaw (Math|Rotator|BreakRotator (Pawn|GetControlRotation (Variables|Default|GetPlayerRef) :!class /Script/Engine.Pawn))))) AxisValue false))

(fn ConstructionScript)

(fn SetFocusonMainMenu
  (bind _returnvalue (Game|GetPlayerController 0))
  (Input|DisableInput _returnvalue _returnvalue)
  (Input|SetInputModeUIOnly self (Variables|/Game/Widgets/PlayerHud.PlayerHud_C|GetMenuWidget (Variables|/Game/Blueprints/Core/ThirdPersonCharacter.ThirdPersonCharacter_C|GetPlayerHUD (Variables|Default|GetPlayerRef))) "DoNotLock")
  (Variables|Default|SetbShowMouseCursor true))

(fn SetGameplayFocus
  (bind _returnvalue (Game|GetPlayerController 0))
  (Input|EnableInput _returnvalue _returnvalue)
  (Input|SetInputModeGameOnly self)
  (Variables|Default|SetbShowMouseCursor false))

(fn SwitchControltoWidget
  (params (Switch :type Boolean) (InWidgetToFocus :type Widget%20Object%20Reference))
  (bind _output_get (Variables|Default|SetbShowMouseCursor Switch))
  (if _output_get
    (Input|SetInputModeGameandUI self InWidgetToFocus "DoNotLock" true)
    (else
      (Input|SetInputModeGameOnly self))))