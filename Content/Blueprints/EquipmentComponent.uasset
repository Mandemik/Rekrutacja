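; Equipment component that tracks the building materials brick, wood and diament in a BuildingItems struct.
; An init event stores a widget reference, and pick events add the given amount to the matching material and copy the new total to that widget.
; DeletBuildingItems subtracts a passed-in set of amounts from all three and refreshes every widget count, with no check against going below zero.
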(event Custom|PickBrick
  (params (BrickValue :type Float%20%28single-precision%29))
  (Variables|Default|SetBuildingItems (Utilities|Struct|MakeBuildRequestStruct (.diament (Variables|Default|GetBuildingItems)) (+ BrickValue (.brick (Variables|Default|GetBuildingItems))) (.wood (Variables|Default|GetBuildingItems))))
  (Variables|/Game/Widgets/EquipmentWidget.EquipmentWidget_C|SetBrickNumber (Variables|Default|GetWidgetRef) (.brick (Variables|Default|GetBuildingItems))))

(event Custom|ComponentInit
  (params (WidgetRef :type Equipment%20Widget%20Object%20Reference))
  (Variables|Default|SetWidgetRef WidgetRef))

(event Custom|PickWood
  (params (WoodValue :type Float%20%28single-precision%29))
  (Variables|Default|SetBuildingItems (Utilities|Struct|MakeBuildRequestStruct (.diament (Variables|Default|GetBuildingItems)) (.brick (Variables|Default|GetBuildingItems)) (+ (.wood (Variables|Default|GetBuildingItems)) WoodValue)))
  (Variables|/Game/Widgets/EquipmentWidget.EquipmentWidget_C|SetWoodNumber (Variables|Default|GetWidgetRef) (.wood (Variables|Default|GetBuildingItems))))

(event Custom|PickDiament
  (params (DiamentValue :type Float%20%28single-precision%29))
  (Variables|Default|SetBuildingItems (Utilities|Struct|MakeBuildRequestStruct (+ DiamentValue (.diament (Variables|Default|GetBuildingItems))) (.brick (Variables|Default|GetBuildingItems)) (.wood (Variables|Default|GetBuildingItems))))
  (Variables|/Game/Widgets/EquipmentWidget.EquipmentWidget_C|SetDiamonNumber (Variables|Default|GetWidgetRef) (.diament (Variables|Default|GetBuildingItems))))

(fn DeletBuildingItems
  (params (ItemToDelete :type Build%20Request%20Struct%20Structure))
  (Variables|Default|SetBuildingItems (Utilities|Struct|MakeBuildRequestStruct (- (.diament (Variables|Default|GetBuildingItems)) (.diament ItemToDelete)) (- (.brick (Variables|Default|GetBuildingItems)) (.brick ItemToDelete)) (- (.wood (Variables|Default|GetBuildingItems)) (.wood ItemToDelete))))
  (Utilities|FlowControl|Sequence
    (:then_0
      (Variables|/Game/Widgets/EquipmentWidget.EquipmentWidget_C|SetBrickNumber (Variables|Default|GetWidgetRef) (.brick (Variables|Default|GetBuildingItems))))
    (:then_1
      (Variables|/Game/Widgets/EquipmentWidget.EquipmentWidget_C|SetDiamonNumber (Variables|Default|GetWidgetRef) (.diament (Variables|Default|GetBuildingItems))))
    (:then_2
      (Variables|/Game/Widgets/EquipmentWidget.EquipmentWidget_C|SetWoodNumber (Variables|Default|GetWidgetRef) (.wood (Variables|Default|GetBuildingItems))))))