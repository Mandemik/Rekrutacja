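; GhostSpawner is an actor that spawns Ghost actors to attack a given target.
; On BeginPlay it adds itself to the GhostSpawner list on ThirdPersonGameMode.
; StartAttack stores the target, spawns a first wave immediately and starts a looping timer at the spawn interval.
; Each wave spawns one Ghost per listed transform, converted against the root's world transform, passing it the target and skipping spawns whose collisions cannot be resolved.
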(event Custom|StartAttack
  (params (MainTarget :type Actor%20Object%20Reference))
  (Variables|Default|SetTargetToAttack MainTarget)
  (CallFunction|SpawnGhosts)
  (Utilities|Time|SetTimerbyEvent (EventDispatchers|CreateEvent :!event Custom|SpawnGhosts) (Variables|Default|GetSpawnFrequence) true))

(event Custom|SpawnGhosts
  (for _array_element (Variables|Default|GetSpawnGhostTransformLiast)
    (Game|SpawnActorfromClass "/Game/Blueprints/AI/Ghost.Ghost_C" (Class|KismetMathLibrary|ConvertTransformtoRelative _array_element (Transformation|GetWorldTransform (Variables|Default|GetDefaultSceneRoot self))) "AdjustIfPossibleButDontSpawnIfColliding" 0 (Variables|Default|GetTargetToAttack) 0)))

(event EventBeginPlay
  (Utilities|Array|Add (Variables|/Game/Blueprints/Core/ThirdPersonGameMode.ThirdPersonGameMode_C|GetGhostSpawner (.AsThird%20Person%20Game%20Mode (Utilities|Casting|CastToThirdPersonGameMode (Game|GetGameMode)))) self))

(fn ConstructionScript)