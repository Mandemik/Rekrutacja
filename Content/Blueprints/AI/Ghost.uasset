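; Ghost AI enemy that attacks a combat target, or its main target when no combat target is valid.
; A HealthComponent drives the widget health bar, with bound events for death and HP changes that destroy the ghost or reveal the bar.
; Attacks apply damage through the target's HealthComponent, gated by a cooldown timer.
; A dynamic material created at construction toggles emissive glow for the aggressive stance; ChangePatrolPointToWorld is empty.
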(event Custom|AttackCooldownFinished
  (Variables|Default|SetCanAtack true))

(event Custom|CustomEvent_0
  (params (CurrentHP :type Float%20%28single-precision%29))
  (if (not (== CurrentHP (Variables|Default|GetHP)))
    (Rendering|SetVisibility (Variables|Default|GetHealBar) true false)))

(event Custom|KillGhost
  (Actor|DestroyActor))

(event EventBeginPlay
  (bind _healthcomponent (Variables|Default|GetHealthComponent))
  (bind _ashealth_bar (Utilities|Casting|CastToHealthBar (UserInterface|GetUserWidgetObject (Variables|Default|GetHealBar))))
  (bind _output_get (Variables|Default|SetHPwidget _ashealth_bar))
  (Variables|/Game/Blueprints/HealthComponent.HealthComponent_C|SetWidgetHP _healthcomponent _output_get)
  (Default|InitComponent _healthcomponent false 0.0)
  (EventDispatchers|BindEventtoYouAreDead _healthcomponent (EventDispatchers|CreateEvent :!event Custom|KillGhost))
  (EventDispatchers|BindEventtoYourCurrentHP _healthcomponent (EventDispatchers|CreateEvent :!event Custom|CustomEvent_0)))

(event EventAttack
  (bind _maintarget (Variables|Default|GetMainTarget))
  (bind _combattarget (Variables|Default|GetCombatTarget))
  (if (Variables|Default|GetCanAtack)
    (Variables|Default|SetCanAtack false)
    (Utilities|Time|SetTimerbyEvent (EventDispatchers|CreateEvent :!event Custom|AttackCooldownFinished) (Variables|Default|GetAttackFrequency))
    (Utilities|IsValid _combattarget
      (:Is%20Valid
        (Default|TakeDamage (Actor|GetComponentbyClass _combattarget "/Game/Blueprints/HealthComponent.HealthComponent_C") 1.0))
      (:Is%20Not%20Valid
        (Utilities|IsValid _maintarget
          (:Is%20Valid
            (Default|TakeDamage (Actor|GetComponentbyClass _maintarget "/Game/Blueprints/HealthComponent.HealthComponent_C") 25.0)))))))

(fn ConstructionScript
  (bind _returnvalue (Rendering|Material|CreateDynamicMaterialInstance (Variables|Character|GetMesh) 0 0 "" :!class /Script/Engine.PrimitiveComponent))
  (Variables|Default|SetEmisiveMaterial _returnvalue))

(fn ChangePatrolPointtoWorld)

(fn ShowAgressiveStance
  (params (State :type Boolean))
  (if State
    (Rendering|Material|SetScalarParameterValue (Variables|Default|GetEmisiveMaterial) "Emissive" 1.0 :!class /Script/Engine.MaterialInstanceDynamic)
    (else
      (Rendering|Material|SetScalarParameterValue (Variables|Default|GetEmisiveMaterial) "Emissive" 0.0 :!class /Script/Engine.MaterialInstanceDynamic))))