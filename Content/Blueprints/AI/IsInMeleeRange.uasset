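; IsInMeleeRange is a behavior tree service that flags whether the AI's target is alive and within melee range.
; On activation, it reads the target actor from the blackboard, checks IsLive on its HealthComponent and compares the pawn's distance against MeleeRange.
; The combined result is written to the BBIsInRange key, with no update on tick.
; A trailing branch repeats the distance check but does nothing.
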(event EventReceiveActivationAI
  (params (OwnerController :type AI%20Controller%20Object%20Reference) (ControlledPawn :type Pawn%20Object%20Reference))
  (bind _meleerange (Variables|Default|GetMeleeRange))
  (bind _bb_target (Variables|Default|GetBB_Target))
  (bind _returnvalue (AI|BehaviorTree|GetBlackboardValueasActor _bb_target))
  (bind _returnvalue_2 (Transformation|GetDistanceTo ControlledPawn _returnvalue))
  (bind _returnvalue_3 (<= _returnvalue_2 _meleerange))
  (Class|BTFunctionLibrary|SetBlackboardValueasBool (Variables|Default|GetBB_IsInRange) (and (Variables|/Game/Blueprints/HealthComponent.HealthComponent_C|GetIsLive (Actor|GetComponentbyClass _returnvalue "/Game/Blueprints/HealthComponent.HealthComponent_C")) _returnvalue_3))
  (if _returnvalue_3
    _))