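; Behavior tree task that picks the next patrol point for a Ghost AI.
; It increments the blackboard patrol index, resetting it to zero only when it already equals the patrol location count.
; It then converts that entry of the Ghost's PatrolDetails locations from the actor's local space to world space, writes it to the next-location blackboard key and finishes successfully.
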(event EventReceiveExecuteAI
  (params (OwnerController :type AI%20Controller%20Object%20Reference) (ControlledPawn :type Pawn%20Object%20Reference))
  (bind _asghost (Utilities|Casting|CastToGhost ControlledPawn))
  (bind _bb_currenpatrolindex (Variables|Default|GetBB_CurrenPatrolIndex))
  (bind _returnvalue (Class|BTFunctionLibrary|GetBlackboardValueasInt _bb_currenpatrolindex))
  (bind _patroldetails (Variables|/Game/Blueprints/AI/Ghost.Ghost_C|GetPatrolDetails _asghost))
  (bind _patrollocation (Variables|/Game/Blueprints/AI/PatrolRot.PatrolRot_C|GetPatrolLocation _patroldetails))
  (if (== _returnvalue (Utilities|Array|Length _patrollocation))
    (Class|BTFunctionLibrary|SetBlackboardValueasInt (Variables|Default|GetBB_CurrenPatrolIndex))
    (else
      (bind _result (Math|Integer|IncrementInt _returnvalue)
        (:%20%20
          (Class|BTFunctionLibrary|SetBlackboardValueasInt (Variables|Default|GetBB_CurrenPatrolIndex) _result)))))
  (AI|BehaviorTree|SetBlackboardValueasVector (Variables|Default|GetBB_NextPatrolLocation) (Math|Transform|TransformLocation (Transformation|GetActorTransform _patroldetails) (Utilities|Array|Get(acopy) _patrollocation _returnvalue)))
  (AI|BehaviorTree|FinishExecute true))