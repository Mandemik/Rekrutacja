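; CheakPlayerThreat is a behavior tree service that flags whether the AI's target is close enough to count as a threat.
; On activation, if the see-player Blackboard key is true, it compares the pawn's distance to the target actor against ThreatRange and writes the result to the in-threat key.
; When the player is not seen, it clears that key.
; The check runs only on activation, with no tick update.
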(event EventReceiveActivationAI
  (params (OwnerController :type AI%20Controller%20Object%20Reference) (ControlledPawn :type Pawn%20Object%20Reference))
  (if (Class|BTFunctionLibrary|GetBlackboardValueasBool (Variables|Default|GetBB_SeePlayer))
    (Class|BTFunctionLibrary|SetBlackboardValueasBool (Variables|Default|GetBB_IsInThreat) (<= (Transformation|GetDistanceTo ControlledPawn (AI|BehaviorTree|GetBlackboardValueasActor (Variables|Default|GetBB_Target))) (Variables|Default|GetThreatRange)))
    (else
      (Class|BTFunctionLibrary|SetBlackboardValueasBool (Variables|Default|GetBB_IsInThreat) false))))