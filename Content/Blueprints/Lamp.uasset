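; Lamp Blueprint with a point light and particle effect that can be switched on or off.
; The SwitchLight event sets both components' active state and visibility, and optionally plays the Zapalanie (ignition) sound at the actor's location when switching on.
; The construction script calls it silently with the TurnOn variable to apply the initial state.
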(event Custom|SwitchLight
  (params (On/Off :type Boolean) (PlaySound :type Boolean))
  (bind _pointlight (Variables|Default|GetPointLight))
  (Components|Activation|SetActive _pointlight On/Off false)
  (Rendering|SetVisibility _pointlight On/Off false)
  (if (and On/Off PlaySound)
    (Audio|PlaySoundatLocation "/Game/Sound/Zapalanie.Zapalanie" (Transformation|GetActorLocation) "0, 0, 0" 1.0 1.0 0.0 0 0 0)))

(fn ConstructionScript
  (CallFunction|SwitchLight (Variables|Default|GetTurnOn) false))