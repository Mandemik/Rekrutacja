(event OnComponentBeginOverlap(Sphere1)
  (params (OverlappedComponent :type Primitive%20Component%20Object%20Reference) (OtherActor :type Actor%20Object%20Reference) (OtherComp :type Primitive%20Component%20Object%20Reference) (OtherBodyIndex :type Integer) (bFromSweep :type Boolean) (SweepResult :type Hit%20Result%20Structure%20%28by%20ref%29))
  (bind _isworking (Variables|Default|GetIsWorking))
  (bind _asghost (Utilities|Casting|CastToGhost OtherActor))
  (if (and (and (not (Variables|Default|GetIsShooting)) _isworking) _isworking)
    (Variables|Default|SetIsShooting true)
    (CallFunction|SetNewTarget _asghost)
    (CallFunction|ShootatTarget)))

(event OnComponentBeginOverlap(BuildInfoTrigger)
  (params (OverlappedComponent :type Primitive%20Component%20Object%20Reference) (OtherActor :type Actor%20Object%20Reference) (OtherComp :type Primitive%20Component%20Object%20Reference) (OtherBodyIndex :type Integer) (bFromSweep :type Boolean) (SweepResult :type Hit%20Result%20Structure%20%28by%20ref%29))
  (if (and (.bSuccess (Utilities|Casting|CastToThirdPersonCharacter OtherActor)) (not (Variables|/Game/Blueprints/TowerUseComponent.TowerUseComponent_C|GetHasBeenBuild (Variables|Default|GetTowerUseComponent))))
    (Rendering|SetVisibility (Variables|Default|GetBuildRequest) true true)))

(event OnComponentEndOverlap(BuildInfoTrigger)
  (params (OverlappedComponent :type Primitive%20Component%20Object%20Reference) (OtherActor :type Actor%20Object%20Reference) (OtherComp :type Primitive%20Component%20Object%20Reference) (OtherBodyIndex :type Integer))
  (if (.bSuccess (Utilities|Casting|CastToThirdPersonCharacter OtherActor))
    (Rendering|SetVisibility (Variables|Default|GetBuildRequest) false true)))

(event Custom|ShootAtTarget
  (bind _shootingtarget (Variables|Default|GetShootingTarget))
  (if (Math|Boolean|ANDBoolean (Variables|Default|GetIsWorking) (Utilities|IsValid _shootingtarget) (Collision|IsOverlappingActor (Variables|Default|GetSphere1) _shootingtarget :!class /Script/Engine.PrimitiveComponent))
    (bind _returnvalue (Utilities|Time|SetTimerbyEvent (EventDispatchers|CreateEvent :!event Custom|GunTowerRotation) 0.05 true))
    (Variables|Default|SetTowerRotationTImer _returnvalue)
    (Default|TakeDamage (Variables|/Game/Blueprints/AI/Ghost.Ghost_C|GetHealthComponent (Variables|Default|GetShootingTarget)) (Variables|Default|GetDamage))
    (if false
      (CallFunction|StopShooting))
    (else
      (CallFunction|StopShooting))))

(event Custom|TowerHasBeenBuild
  (if (not (Variables|Default|GetIsWorking))
    (Variables|Default|SetIsWorking true)
    (CallFunction|SetVisualWorkingTower)
    (Default|CallTowerBuild)
    (bind _closestenemy (CallFunction|FindClosestTarget))
    (Utilities|IsValid _closestenemy
      (:Is%20Valid
        (CallFunction|SetNewTarget _closestenemy)))))

(event Custom|GunTowerRotation
  (bind _stupidroot (Variables|Default|GetStupidRoot))
  (bind _shootingtarget (Variables|Default|GetShootingTarget))
  (bind _returnvalue (Transformation|GetWorldRotation _stupidroot))
  (Utilities|IsValid _shootingtarget
    (:Is%20Valid
      (Transformation|SetRelativeRotation _stupidroot (Math|Rotator|MakeRotator (.roll _returnvalue) (.pitch _returnvalue) (.yaw (Math|Rotator|FindLookatRotation (Transformation|GetWorldLocation (Variables|Default|GetStupidRoot)) (Transformation|GetActorLocation _shootingtarget)))) false false))
    (:Is%20Not%20Valid
      (Utilities|Time|ClearandInvalidateTimerbyHandle (Variables|Default|GetTowerRotationTImer)))))

(event Custom|TowerHasBeenDestory
  (if (Variables|Default|GetIsWorking)
    (Rendering|SetVisibility (Variables|Default|GetHealBar) false false)
    (Utilities|Time|ClearandInvalidateTimerbyHandle (Variables|Default|GetShootingTimmer))
    (Utilities|Time|ClearandInvalidateTimerbyHandle (Variables|Default|GetTowerRotationTImer))
    (CallFunction|SetVisualNotWorkingTower)
    (Variables|Default|SetIsWorking false)
    (Default|CallTowerDestroy)))

(event EventBeginPlay
  (bind _healthcomponent (Variables|Default|GetHealthComponent))
  (Variables|/Game/Blueprints/HealthComponent.HealthComponent_C|SetWidgetHP _healthcomponent (.AsHealth%20Bar (Utilities|Casting|CastToHealthBar (UserInterface|GetUserWidgetObject (Variables|Default|GetHealBar)))))
  (Default|InitComponent (Variables|Default|GetTowerUseComponent) _healthcomponent self)
  (if (Variables|Default|GetIsWorking)
    (Default|InitComponent _healthcomponent false 0.0)
    (else
      (Default|InitComponent _healthcomponent true 0.0)))
  (EventDispatchers|BindEventtoYouAreDead (Variables|Default|GetHealthComponent) (EventDispatchers|CreateEvent :!event Custom|TowerHasBeenDestory))
  (CallFunction|SetBuildWidgetParamet))

(fn ConstructionScript
  (Components|Sphere|SetSphereRadius (Variables|Default|GetSphere1) (Variables|Default|GetTowerRange) true)
  (if (Variables|Default|GetIsWorking)
    (CallFunction|SetVisualWorkingTower)
    (else
      (CallFunction|SetVisualNotWorkingTower))))

(fn FindClosestTarget
  (bind _sphere1 (Variables|Default|GetSphere1))
  (bind _overlappingactors (Collision|GetOverlappingActors _sphere1 "/Game/Blueprints/AI/Ghost.Ghost_C" :!class /Script/Engine.PrimitiveComponent))
  (if (== (Utilities|Array|Length _overlappingactors) 0)
    (return 0)
    (else
      (for _array_element _overlappingactors
        (if (< (Transformation|GetDistanceTo _array_element) (LocalVariables|GetClosestDistance))
          (LocalVariables|SetClosestDistance (Transformation|GetDistanceTo _array_element))
          (LocalVariables|SetClosestTarget (.AsGhost (Utilities|Casting|CastToGhost _array_element)))))
      (return (LocalVariables|GetClosestTarget)))))

(fn SetNewTarget
  (params (ShootingTarget :type Ghost%20Object%20Reference))
  (Variables|Default|SetShootingTarget ShootingTarget)
  (bind _returnvalue (Utilities|Time|SetTimerbyEvent (EventDispatchers|CreateEvent :!event Custom|ShootAtTarget) (Variables|Default|GetFrequence) true))
  (Variables|Default|SetShootingTimmer _returnvalue))

(fn SetVisualWorkingTower
  (bind _cube (Variables|Default|GetCube))
  (Rendering|Material|SetMaterial _cube 0 (Variables|Default|GetWorkingTowerMaterial))
  (Components|StaticMesh|SetStaticMesh _cube (Variables|Default|GetWorkingTowerMesh))
  (Rendering|SetVisibility (Variables|Default|GetStupidRoot) true true)
  (Rendering|SetVisibility (Variables|Default|GetHealBar) true false)
  (return))

(fn SetVisualNotWorkingTower
  (bind _cube (Variables|Default|GetCube))
  (Rendering|Material|SetMaterial _cube 0 (Variables|Default|GetNotWorkingTowerMaterial))
  (Components|StaticMesh|SetStaticMesh _cube (Variables|Default|GetNotWorkingTowerMesh))
  (Rendering|SetVisibility (Variables|Default|GetStupidRoot) false true)
  (Rendering|SetVisibility (Variables|Default|GetHealBar) false false))

(fn StopShooting
  (Utilities|Time|ClearandInvalidateTimerbyHandle (Variables|Default|GetShootingTimmer))
  (Utilities|Time|ClearandInvalidateTimerbyHandle (Variables|Default|GetTowerRotationTImer))
  (Variables|Default|SetShootingTarget 0)
  (bind _closestenemy (CallFunction|FindClosestTarget))
  (Utilities|IsValid _closestenemy
    (:Is%20Valid
      (CallFunction|SetNewTarget _closestenemy))
    (:Is%20Not%20Valid
      (Variables|Default|SetIsShooting false))))

(fn SetBuildWidgetParamet
  (bind _buildrequest (Variables|Default|GetBuildRequest))
  (bind _towerusecomponent (Variables|Default|GetTowerUseComponent))
  (bind _returnvalue (UserInterface|GetUserWidgetObject _buildrequest))
  (bind _buildrequest_2 (Variables|/Game/Blueprints/TowerUseComponent.TowerUseComponent_C|GetBuildRequest _towerusecomponent))
  (bind _asequipment_widget (Utilities|Casting|CastToEquipmentWidget _returnvalue))
  (Variables|/Game/Widgets/EquipmentWidget.EquipmentWidget_C|SetDiamonNumber _asequipment_widget (.diament _buildrequest_2))
  (Variables|/Game/Widgets/EquipmentWidget.EquipmentWidget_C|SetBrickNumber _asequipment_widget (.brick _buildrequest_2))
  (Variables|/Game/Widgets/EquipmentWidget.EquipmentWidget_C|SetWoodNumber _asequipment_widget (.wood _buildrequest_2)))