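; Stone altar actor that receives memories carried by the player's ThirdPersonCharacter and displays items on itself.
; When the character enters its Box trigger, it registers itself on the character and calls that character's deploy-memory function if a memory is being carried.
; AddVisualItem spawns a static mesh component and snaps it to a numbered socket on the altar mesh, incrementing a counter for the next slot.
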(event OnComponentBeginOverlap(Box)
  (params (OverlappedComponent :type Primitive%20Component%20Object%20Reference) (OtherActor :type Actor%20Object%20Reference) (OtherComp :type Primitive%20Component%20Object%20Reference) (OtherBodyIndex :type Integer) (bFromSweep :type Boolean) (SweepResult :type Hit%20Result%20Structure%20%28by%20ref%29))
  (bind _asthird_person_character (Utilities|Casting|CastToThirdPersonCharacter OtherActor))
  (Variables|/Game/Blueprints/Core/ThirdPersonCharacter.ThirdPersonCharacter_C|SetStoneAltar _asthird_person_character self)
  (if (Variables|/Game/Blueprints/Core/ThirdPersonCharacter.ThirdPersonCharacter_C|GetCarringMemory _asthird_person_character)
    (Default|CallDeployMemory _asthird_person_character)))

(event Custom|AddVisualItem
  (params (NewMesh :type Static%20Mesh%20Object%20Reference) (SocketName :type Name))
  (bind _returnvalue (AddComponent|AddStaticMeshComponent false))
  (Components|StaticMesh|SetStaticMesh _returnvalue NewMesh)
  (Transformation|AttachComponentToComponent _returnvalue (Variables|Debug|GetStaticMeshComponent) (Utilities|Name|MakeLiteralName (Utilities|String|StringToName (Utilities|String|Append (Utilities|String|ToString(Name) SocketName) (Utilities|String|ToString(Integer) (Variables|Default|GetComponentNumber))))) "SnapToTarget" "SnapToTarget" "SnapToTarget" true)
  (Math|Integer|IncrementInt (Variables|Default|GetComponentNumber)))

(event EventBeginPlay)

(event Collision|EventActorBeginOverlap
  (params (OtherActor :type Actor%20Object%20Reference)))

(event EventTick
  (params (DeltaSeconds :type Float%20%28single-precision%29)))

(fn ConstructionScript)